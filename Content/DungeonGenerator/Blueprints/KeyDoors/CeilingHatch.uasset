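; Ceiling hatch for the dungeon generator that can start locked and lowers four platforms from overhead when opened.
; An overlapping BP_DoorKey with the desired tag unlocks it and is optionally destroyed, while any non-key actor triggers it if already unlocked.
; A Timeline drives each platform's height on its own track, and the construction script applies a shared material to all four.
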(event OnComponentBeginOverlap(Box)
  (params (OverlappedComponent :type Primitive%20Component%20Object%20Reference) (OtherActor :type Actor%20Object%20Reference) (OtherComp :type Primitive%20Component%20Object%20Reference) (OtherBodyIndex :type Integer) (bFromSweep :type Boolean) (SweepResult :type Hit%20Result%20Structure%20%28by%20ref%29))
  (bind _asbp_door_key (Utilities|Casting|CastToBP_DoorKey OtherActor)
    (:then
      (if (Actor|ActorHasTag OtherActor (Variables|Default|GetDesiredKeyTag))
        (CallFunction|Unlock)
        (if (Variables|Default|GetConsumeKey?)
          (Actor|DestroyActor _asbp_door_key))))
    (:CastFailed
      (if (not (Variables|Default|GetStartLocked?))
        (bind (_direction _platform1 _platform2 _platform3 _platform4) (Timeline|Timeline Play)
          (:Update
            (Transformation|SetRelativeLocation (Variables|Default|GetPlatform1) (Math|Vector|MakeVector 125.0 -125.0 (- 5e+02 _platform1)) false false)
            (Transformation|SetRelativeLocation (Variables|Default|GetPlatform2) (Math|Vector|MakeVector 125.0 125.0 (- 5e+02 _platform2)) false false)
            (Transformation|SetRelativeLocation (Variables|Default|GetPlatform3) (Math|Vector|MakeVector -125.0 125.0 (- 5e+02 _platform3)) false false)
            (Transformation|SetRelativeLocation (Variables|Default|GetPlatform4) (Math|Vector|MakeVector -125.0 -125.0 (- 5e+02 _platform4)) false false)))))))

(event Custom|Unlock
  (Variables|Default|SetStartLocked? false)
  (bind (_direction _platform1 _platform2 _platform3 _platform4) (Timeline|Timeline Play)
    (:Update
      (Transformation|SetRelativeLocation (Variables|Default|GetPlatform1) (Math|Vector|MakeVector 125.0 -125.0 (- 5e+02 _platform1)) false false)
      (Transformation|SetRelativeLocation (Variables|Default|GetPlatform2) (Math|Vector|MakeVector 125.0 125.0 (- 5e+02 _platform2)) false false)
      (Transformation|SetRelativeLocation (Variables|Default|GetPlatform3) (Math|Vector|MakeVector -125.0 125.0 (- 5e+02 _platform3)) false false)
      (Transformation|SetRelativeLocation (Variables|Default|GetPlatform4) (Math|Vector|MakeVector -125.0 -125.0 (- 5e+02 _platform4)) false false))))

(event EventBeginPlay)

(event Collision|EventActorBeginOverlap
  (params (OtherActor :type Actor%20Object%20Reference)))

(event EventTick
  (params (DeltaSeconds :type Float%20%28single-precision%29)))

(fn ConstructionScript
  (Rendering|Material|SetMaterial (Variables|Default|GetPlatform1) 0 (Variables|Default|GetMaterial)))