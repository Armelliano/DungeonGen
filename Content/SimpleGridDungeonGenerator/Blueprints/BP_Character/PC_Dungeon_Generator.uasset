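; Player controller for the dungeon generator, adding debug-style keys for mouse control and dungeon regeneration.
; M flip-flops between a visible cursor with Game and UI input and Game Only input without the cursor.
; R passes through events labeled as client and server RPCs, then finds BP_Dungeon_Generator in the level and tells it to regenerate.
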(event Custom|[%20RPC%20-%20CLIENT%20]%20R%20to%20Regerate%20Dungeon
  ;[1 1 1] REGENERATE DUNGEON IF "R" IS PRESSED
  ;;[1 1 1] Replication System
  (CallFunction|[RPC-SERVER]RtoRegerateDungeon))

(event Custom|[%20RPC%20-%20SERVER%20]%20R%20to%20Regerate%20Dungeon
  ;[1 1 1] REGENERATE DUNGEON IF "R" IS PRESSED
  ;;[1 1 1] Replication System
  (CallFunction|RtoRegerateDungeon))

(event Custom|R%20to%20Regerate%20Dungeon
  ;[1 1 1] REGENERATE DUNGEON IF "R" IS PRESSED
  (bind _returnvalue (Actor|GetActorOfClass "/Game/SimpleGridDungeonGenerator/Blueprints/BP_Dungeon_Generator.BP_Dungeon_Generator_C"))
  (Utilities|IsValid _returnvalue
    (:Is%20Valid
      (Default|REGENERATEDUNGEON _returnvalue))))

(event Input|KeyboardEvents|M
  (params (Key :type Key%20Structure :default "None"))
  ;[1 1 1] If "M" Is Pressed Then Show The Mouse
  (:Pressed
    (Utilities|FlowControl|FlipFlop
      (:A
        (Variables|Default|SetbShowMouseCursor true)
        (Input|SetInputModeGameandUI (Game|GetPlayerController 0) 0 "DoNotLock" true))
      (:B
        (Variables|Default|SetbShowMouseCursor false)
        (Input|SetInputModeGameOnly (Game|GetPlayerController 0))))))

(event Input|KeyboardEvents|R
  (params (Key :type Key%20Structure :default "None"))
  ;[1 1 1] REGENERATE DUNGEON IF "R" IS PRESSED
  ;;[1 1 1] Replication System
  (:Pressed
    (CallFunction|[RPC-CLIENT]RtoRegerateDungeon)))

(fn ConstructionScript)