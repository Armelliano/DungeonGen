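; Actor component on spawned dungeon rooms that finds which neighboring grid directions are free for the grid dungeon generator.
; On BeginPlay it runs through client and server RPCs, then takes room size and debug draw from BP_Dungeon_Generator.
; Four line traces prune blocked directions, passing the remaining list to the generator or calling CollisionDetected if none remain.
; A vertical trace at the room's position sets the generator's Collision flag.
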(event Custom|[%20RPC%20-%20SERVER%20]%20Generation%20Component
  ;[1 0 0] Activate When A Room Is Spawned
  (CallFunction|GenerationComponent))

(event Custom|[%20RPC%20-%20CLIENT%20]%20Generation%20Component
  ;[1 1 1] Server Comunication
  (CallFunction|[RPC-SERVER]GenerationComponent))

(event Custom|Generation%20Component
  (Variables|Default|SetRoom%20Position (Transformation|GetActorLocation (Components|GetOwner)))
  (Utilities|FlowControl|Sequence
    (:then_0
      ;[1 1 1] Set Room Size As Test Vector Size From BP_Dungeon_Generator
      (bind _returnvalue (Actor|GetActorOfClass "/Game/SimpleGridDungeonGenerator/Blueprints/BP_Dungeon_Generator.BP_Dungeon_Generator_C"))
      (Utilities|IsValid _returnvalue
        (:Is%20Valid
          (Variables|Default|SetTest%20Vector%20Size (Variables|/Game/SimpleGridDungeonGenerator/Blueprints/BP_Dungeon_Generator.BP_Dungeon_Generator_C|GetRoom%20Size _returnvalue))
          (Variables|Default|SetDebug%20Lines%20? (Variables|/Game/SimpleGridDungeonGenerator/Blueprints/BP_Dungeon_Generator.BP_Dungeon_Generator_C|GetRoom%20Z%20Collision%20Debug%20Strings%20%28%20Supperpositions%20%29 _returnvalue)))))
    (:then_1
      ;[0 1 0.5] Line Trace A Collision Test To Left, Right, Forward and Backward
      ;;[1 1 1] Test Path Posibilities 0
      (bind _returnvalue_2 (Collision|LineTraceByChannel (Variables|Default|GetRoom%20Position) (Math|Vector|MakeVector (+ (.X (Math|Vector|BreakVector (Variables|Default|GetRoom%20Position))) (Variables|Default|GetTest%20Vector%20Size)) (.Y (Math|Vector|BreakVector (Variables|Default|GetRoom%20Position))) (.Z (Math|Vector|BreakVector (Variables|Default|GetRoom%20Position)))) "TraceTypeQuery1" false 0 (Variables|Default|GetDebug%20Lines%20?)))
      (if _returnvalue_2
        (Utilities|Array|RemoveItem (Variables|Default|GetList%20Of%20Posibilities) 0)))
    (:then_2
      ;;[1 1 1] Test Path Posibilities 1
      (bind _returnvalue_3 (Collision|LineTraceByChannel (Variables|Default|GetRoom%20Position) (Math|Vector|MakeVector (- (.X (Math|Vector|BreakVector (Variables|Default|GetRoom%20Position))) (Variables|Default|GetTest%20Vector%20Size)) (.Y (Math|Vector|BreakVector (Variables|Default|GetRoom%20Position))) (.Z (Math|Vector|BreakVector (Variables|Default|GetRoom%20Position)))) "TraceTypeQuery1" false 0 (Variables|Default|GetDebug%20Lines%20?)))
      (if _returnvalue_3
        (Utilities|Array|RemoveItem (Variables|Default|GetList%20Of%20Posibilities) 1)))
    (:then_3
      ;;[1 1 1] Test Path Posibilities 2
      (bind _returnvalue_4 (Collision|LineTraceByChannel (Variables|Default|GetRoom%20Position) (Math|Vector|MakeVector (.X (Math|Vector|BreakVector (Variables|Default|GetRoom%20Position))) (+ (.Y (Math|Vector|BreakVector (Variables|Default|GetRoom%20Position))) (Variables|Default|GetTest%20Vector%20Size)) (.Z (Math|Vector|BreakVector (Variables|Default|GetRoom%20Position)))) "TraceTypeQuery1" false 0 (Variables|Default|GetDebug%20Lines%20?)))
      (if _returnvalue_4
        (Utilities|Array|RemoveItem (Variables|Default|GetList%20Of%20Posibilities) 2)))
    (:then_4
      ;;[1 1 1] Test Path Posibilities 3
      (bind _returnvalue_5 (Collision|LineTraceByChannel (Variables|Default|GetRoom%20Position) (Math|Vector|MakeVector (.X (Math|Vector|BreakVector (Variables|Default|GetRoom%20Position))) (- (.Y (Math|Vector|BreakVector (Variables|Default|GetRoom%20Position))) (Variables|Default|GetTest%20Vector%20Size)) (.Z (Math|Vector|BreakVector (Variables|Default|GetRoom%20Position)))) "TraceTypeQuery1" false 0 (Variables|Default|GetDebug%20Lines%20?)))
      (if _returnvalue_5
        (Utilities|Array|RemoveItem (Variables|Default|GetList%20Of%20Posibilities) 3)))
    (:then_5
      ;[0 1 0.5] If A Room Detect A collision
      (if (Utilities|Array|IsEmpty (Variables|Default|GetList%20Of%20Posibilities))
        (bind _returnvalue_6 (Actor|GetActorOfClass "/Game/SimpleGridDungeonGenerator/Blueprints/BP_Dungeon_Generator.BP_Dungeon_Generator_C"))
        (Default|CollisionDetected _returnvalue_6)))
    (:then_6
      ;[1 1 1] Set The available Path To "Dungeon_Generator_BP"
      (bind _returnvalue_7 (Actor|GetActorOfClass "/Game/SimpleGridDungeonGenerator/Blueprints/BP_Dungeon_Generator.BP_Dungeon_Generator_C"))
      (Utilities|IsValid _returnvalue_7
        (:Is%20Valid
          (Variables|/Game/SimpleGridDungeonGenerator/Blueprints/BP_Dungeon_Generator.BP_Dungeon_Generator_C|SetList%20Of%20Posibilities _returnvalue_7 (Variables|Default|GetList%20Of%20Posibilities)))))
    (:then_7
      ;[0 1 0.5] Line Trace A Collision Test At The Exact Same Place Of The Room
      (bind _returnvalue_8 (Collision|LineTraceByChannel (Math|Vector|MakeVector (.X (Math|Vector|BreakVector (Variables|Default|GetRoom%20Position))) (.Y (Math|Vector|BreakVector (Variables|Default|GetRoom%20Position))) (+ (.Z (Math|Vector|BreakVector (Variables|Default|GetRoom%20Position))) 3e+02)) (Math|Vector|MakeVector (.X (Math|Vector|BreakVector (Variables|Default|GetRoom%20Position))) (.Y (Math|Vector|BreakVector (Variables|Default|GetRoom%20Position))) (+ (.Z (Math|Vector|BreakVector (Variables|Default|GetRoom%20Position))) -3e+02)) "TraceTypeQuery1" false 0 (Variables|Default|GetDebug%20Lines%20?) true "(R=1.000000,G=0.000000,B=0.000000,A=1.000000)" "(R=0.000000,G=1.000000,B=0.000000,A=1.000000)" 2e+01))
      (bind _returnvalue_9 (Actor|GetActorOfClass "/Game/SimpleGridDungeonGenerator/Blueprints/BP_Dungeon_Generator.BP_Dungeon_Generator_C"))
      (Utilities|IsValid _returnvalue_9
        (:Is%20Valid
          (if _returnvalue_8
            (Variables|/Game/SimpleGridDungeonGenerator/Blueprints/BP_Dungeon_Generator.BP_Dungeon_Generator_C|SetCollision%20? _returnvalue_9 true)
            (else
              (Variables|/Game/SimpleGridDungeonGenerator/Blueprints/BP_Dungeon_Generator.BP_Dungeon_Generator_C|SetCollision%20? _returnvalue_9 false))))))))

(event EventBeginPlay
  ;[1 1 1] Server Comunication
  (CallFunction|[RPC-CLIENT]GenerationComponent))