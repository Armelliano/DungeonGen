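; Procedural maze actor that rebuilds a seeded tile maze in its Construction Script and moves PlayerStart to a randomly picked dead end.
; GenerateMaze carves paths with a randomized depth-first backtracker, stepping two tiles at a time with bridge tiles between and recording dead ends.
; SpawnMazeMeshes turns the tile sets into mesh instances through InstanceManager: floors, end tiles, random walls, corner fillers, and roofs over unused cells.
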(fn ConstructionScript
  (bind _tilesize (Variables|Default|GetTileSize))
  ;[1 1 1] If not work change value on AddNeighbourLoc and BackTrack -> see note
  ;;[1 1 1] Populate maze with meshes
  (Class|BPIInstanceManager|RemoveAllInstances(Message) (Variables|Default|GetInstanceManager))
  (Variables|Default|SetSize (Utilities|Struct|MakeIntPoint (* (/ (.x (Variables|Default|GetSize)) 2) 2) (* (/ (.y (Variables|Default|GetSize)) 2) 2)))
  (bind (_pathtiles_out _endpath_out) (CallFunction|GenerateMaze (Variables|Default|GetSeed) (Variables|Default|GetSize)))
  (Variables|Default|SetPath%20Tiles _pathtiles_out)
  (Variables|Default|SetEnd%20Path _endpath_out)
  (CallFunction|SpawnMazeMeshes)
  ;;[1 1 1] Find a random EndPath tile and move PlayerStart to those coordinates
  (bind _result (Utilities|Set|ToArray _endpath_out))
  (if (> (Utilities|Array|Length _result) 0)
    (Utilities|Set|Remove (Variables|Default|GetEnd%20Path) (Utilities|Array|Get(acopy) _result (Math|Random|RandomIntegerinRange 0 (Utilities|Array|Length _result))))
    (Transformation|SetActorTransform (Variables|Default|GetPlayerStart) (Math|Transform|MakeTransform (Math|Vector|MakeVector (* (.X (Utilities|Struct|BreakIntPoint (Utilities|Array|Get(acopy) _result (Math|Random|RandomIntegerinRange 0 (Utilities|Array|Length _result))))) _tilesize) (* (.Y (Utilities|Struct|BreakIntPoint (Utilities|Array|Get(acopy) _result (Math|Random|RandomIntegerinRange 0 (Utilities|Array|Length _result))))) _tilesize) 1.2e+02) "0, 0, 0" "1.000000,1.000000,1.000000"))))

(fn GenerateMaze
  (params (Seed :type Integer) (Size :type Int%20Point%20Structure))
  (Math|Random|SetRandomStreamSeed (LocalVariables|GetRandStream) Seed)
  (LocalVariables|SetL_Size Size) ; Know the lenght size
  (bind _output_get (LocalVariables|SetStartingLoc (Utilities|GetRandLocinBounds (LocalVariables|GetL_Size) (LocalVariables|GetRandStream)))) ; Set random position as start position
  (LocalVariables|SetCurrentLoc _output_get) ; Set current position equal to start position
  ;[1 1 1] Repeat control until there left no tiles to check
  (CallFunction|AddNeighbourLoc (LocalVariables|GetL_Size) (LocalVariables|GetRandStream) (LocalVariables|GetCurrentLoc) (LocalVariables|GetPathTiles) (LocalVariables|GetBridgeTiles) (LocalVariables|GetToCheck) (LocalVariables|GetEndPaths) :!label _label) ; Check next neighbour tile
  ;;[1 1 1] If there are tiles to check (>0) return the tile, elsewhere return the list of valid path tiles and end-path tile
  (if (> (Utilities|Set|Length (LocalVariables|GetToCheck)) 0)
    (CallFunction|BackTrack (LocalVariables|GetCurrentLoc) (LocalVariables|GetToCheck) (LocalVariables|GetBridgeTiles) (LocalVariables|GetPathTiles))
    (goto _label)
    (else
      (return (LocalVariables|GetPathTiles) (LocalVariables|GetEndPaths)))))

(fn AddNeighbourLoc
  (params (Size :type Int%20Point%20Structure%20%28by%20ref%29) (RandStream :type Random%20Stream%20Structure%20%28by%20ref%29) (CurrentLoc :type Int%20Point%20Structure%20%28by%20ref%29) (PathTiles :type Set%20of%20Int%20Point%20Structures) (BridgeTiles :type Set%20of%20Int%20Point%20Structures) (ToCheck :type Set%20of%20Int%20Point%20Structures) (EndPaths :type Set%20of%20Int%20Point%20Structures))
  (LocalVariables|SetNeighbourIndex (Math|Random|RandomIntegerinRangefromStream RandStream 0 3))
  (if (Utilities|CheckIsValidLoc (.Floor (Utilities|GetNeighbourandBridge CurrentLoc (LocalVariables|GetNeighbourIndex))) Size PathTiles BridgeTiles) :!label _label
    ;[1 1 1] If true, set the current tile as a possible path or bridge tile and save it
    (Utilities|Set|Add PathTiles (.Floor (Utilities|GetNeighbourandBridge CurrentLoc (LocalVariables|GetNeighbourIndex))))
    (Utilities|Set|Add BridgeTiles (.Bridge (Utilities|GetNeighbourandBridge CurrentLoc (LocalVariables|GetNeighbourIndex))))
    (Utilities|Set|Add ToCheck (.Floor (Utilities|GetNeighbourandBridge CurrentLoc (LocalVariables|GetNeighbourIndex))))
    (CallFunction|AddNeighbourLoc Size RandStream (.Floor (Utilities|GetNeighbourandBridge CurrentLoc (LocalVariables|GetNeighbourIndex))) PathTiles BridgeTiles ToCheck EndPaths)
    (else
      ;[1 1 1] Else, if NeighbourIndex value equal 4, set NeighbourIndex value to 0, elsewhere increase it by 1, than re-check tile with new value
      (Utilities|DoN+ 4
        (:Exit
          (LocalVariables|SetNeighbourIndex (Math|Integer|SelectInt 0 (+ (LocalVariables|GetNeighbourIndex) 1) (> (+ (LocalVariables|GetNeighbourIndex) 1) 3)))
          (goto _label))
        (:OverNth
          ;[1 1 1] If it's a end-path tile, save it to end-path tile list
          (bind _count (CallFunction|GetNeighbourCount CurrentLoc PathTiles))
          (if (== _count 1)
            (Utilities|Set|Add EndPaths CurrentLoc)))))))

(fn GetNeighbourCount
  (params (CurrentLoc :type Int%20Point%20Structure%20%28by%20ref%29) (PathTiles :type Set%20of%20Int%20Point%20Structures))
  ;[1 1 1] Check if target tiles is the end of the path and return the value of neighbour tiles already in use
  (for _array_element (Utilities|GetNeighbourLoc CurrentLoc 1)
    (if (Utilities|Set|Contains PathTiles _array_element)
      (Math|Integer|IncrementInt (LocalVariables|GetCounter))))
  (return (LocalVariables|GetCounter)))

(fn BackTrack
  (params (CurrentTIle :type Int%20Point%20Structure%20%28by%20ref%29) (ToCheck :type Set%20of%20Int%20Point%20Structures) (BridgeTIles :type Set%20of%20Int%20Point%20Structures) (PathTiles :type Set%20of%20Int%20Point%20Structures))
  ;[1 1 1] Clear the list of tiles from in reverse order (from last to first)
  (bind _result (Utilities|Set|ToArray ToCheck))
  (if (> (Utilities|Array|Length _result) 0)
    (|SetBy-RefVar CurrentTIle (Utilities|Array|Get(acopy) _result (Utilities|Array|LastIndex _result)))
    (Utilities|Set|Remove ToCheck (Utilities|Array|Get(acopy) _result (Utilities|Array|LastIndex _result)))
    (bind _result_2 (Utilities|Set|ToArray BridgeTIles)))
  (if (> (Utilities|Array|Length _result_2) 0)
    (Utilities|Set|Add PathTiles (Utilities|Array|Get(acopy) _result_2 (Utilities|Array|LastIndex _result_2)))
    (Utilities|Set|Remove BridgeTIles (Utilities|Array|Get(acopy) _result_2 (Utilities|Array|LastIndex _result_2)))))

(fn SpawnMazeMeshes
  (bind _size (Variables|Default|GetSize))
  ;[1 1 1] Loop through each row and each column and check the cell state
  (for _index (range 0 (.x _size))
    (for _index_2 (range 0 (.y _size))
      (bind _output_get (LocalVariables|SetLoopLoc (Utilities|Struct|MakeIntPoint _index _index_2)))
      (if (Utilities|Set|Contains (Variables|Default|GetPath%20Tiles) _output_get)
        ;;[1 1 1] Add different meshes whether the path tile is an end tile or not
        (Class|BPIInstanceManager|AddNewMeshInstance(Message) (Variables|Default|GetInstanceManager) (select (Utilities|Set|Contains (Variables|Default|GetEnd%20Path) (LocalVariables|GetLoopLoc)) "/Game/Blueprints/Mesh/SM_Ground_End.SM_Ground_End" "/Game/Blueprints/Mesh/SM_Ground_Normal.SM_Ground_Normal") (Utilities|BuildTileLoc (LocalVariables|GetLoopLoc) 0.0))
        ;;[1 1 1] Position the wall mesh based on the orientation of the tiles, randomizing the wall mesh by choosing it from those possible
        (for (_array_element _array_index) (Utilities|GetNeighbourLoc (LocalVariables|GetLoopLoc) 1)
          (LocalVariables|SetLoopIndex _array_index)
          (Utilities|Array|SetArrayElem (LocalVariables|GetSegmentIndex) (LocalVariables|GetLoopIndex) (Utilities|Set|Contains (Variables|Default|GetPath%20Tiles) _array_element) true)
          (if (not (Utilities|Set|Contains (Variables|Default|GetPath%20Tiles) _array_element))
            (Class|BPIInstanceManager|AddNewMeshInstance(Message) (Variables|Default|GetInstanceManager) (Utilities|Select :Index (Math|Random|RandomIntegerinRangefromStream (LocalVariables|GetRandStream) 0 3) :Option%200 "/Game/Blueprints/Mesh/SM_Wall_Flat.SM_Wall_Flat" :Option%201 "/Game/Blueprints/Mesh/SM_Wall_Boxx1.SM_Wall_Boxx1" :Option%202 "/Game/Blueprints/Mesh/SM_Wall_Box2.SM_Wall_Box2" :Option%203 "/Game/Blueprints/Mesh/SM_Wall_Box3.SM_Wall_Box3") (Utilities|BuildTileLoc (LocalVariables|GetLoopLoc) 0.0 (LocalVariables|GetLoopIndex)))))
        ;;[1 1 1] Place corner meshes to fill holes between two corner walls
        (for (_array_element_2 _array_index_2) (LocalVariables|GetSegmentIndex)
          (LocalVariables|SetLoopIndex _array_index_2)
          (if (and _array_element_2 (Utilities|Array|Get(acopy) (LocalVariables|GetSegmentIndex) (Math|Integer|SelectInt (Utilities|Array|LastIndex (LocalVariables|GetSegmentIndex)) (- (LocalVariables|GetLoopIndex) 1) (< (- (LocalVariables|GetLoopIndex) 1) 0))))
            (Class|BPIInstanceManager|AddNewMeshInstance(Message) (Variables|Default|GetInstanceManager) "/Game/Blueprints/Mesh/SM_Wall_Corner.SM_Wall_Corner" (Utilities|BuildTileLoc (LocalVariables|GetLoopLoc) 0.0 (LocalVariables|GetLoopIndex)))))
        (else
          ;;[1 1 1] Add roof mesh over the unused tiles
          (Class|BPIInstanceManager|AddNewMeshInstance(Message) (Variables|Default|GetInstanceManager) "/Game/Blueprints/Mesh/SM_Roof.SM_Roof" (Utilities|BuildTileLoc (LocalVariables|GetLoopLoc) 4e+02)))))))